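; BP_Pacman is the Pacman pawn Blueprint, handling switching between normal and power-up movement.
; On BeginPlay it applies normal speed and acceleration to its FloatingPawnMovement component.
; ApplyPowerUpMovement sets the boosted values, then fires the PowerUpeffect event, which waits PowerUpDuration before restoring normal movement.
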(event `self.ReceiveBeginPlay`
  (`self.Apply Normal Movement`))

(event `PowerUp effect`
  (`KismetSystemLibrary.Delay` (`self.PowerUp Duration`))
  (`self.Apply Normal Movement`))

(fn `Apply Normal Movement`
  (bind _floatingpawnmovement (`self.FloatingPawnMovement`))
  (`|ExecutionSequence`
    (:`then_0`
      (set `FloatingPawnMovement.MaxSpeed` (`self.Normal speed`) _floatingpawnmovement))
    (:`then_1`
      (set `FloatingPawnMovement.Acceleration` (`self.Normal acceleration`) _floatingpawnmovement))))

(fn `Apply PowerUp Movement`
  (bind _floatingpawnmovement (`self.FloatingPawnMovement`))
  (`|ExecutionSequence`
    (:`then_0`
      (set `FloatingPawnMovement.MaxSpeed` (`self.PowerUp speed`) _floatingpawnmovement))
    (:`then_1`
      (set `FloatingPawnMovement.Acceleration` (`self.PowerUp acceleration`) _floatingpawnmovement))
    (:`then_2`
      (`self.PowerUp effect`))))

(fn `UserConstructionScript`)