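; BP_Enemy is the Pac-Man enemy that chases the player and restarts Level_01 when it hits them.
; It idles for two seconds on BeginPlay before hunting, and each state change event retargets its AI controller: Idle stops movement, any other state moves toward the player pawn.
; A sphere hit on BP_Pacman teleports Pac-Man far away, idles the enemy and reloads the level after a short delay.
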(event `Event State Changed SetUp`
  (add `self.StateChangedEvent` (delegate `Event State Changed`)))

(event `Event State Changed` :!signature `self.StateChangedEvent`
  (params (NewState :type "EEnemyState Enum" :default "Default"))
  (`self.UpdateMovementTarget`))

(event `self.ReceiveBeginPlay`
  (`self.Event State Changed SetUp`)
  (`self.Idle`)
  (`KismetSystemLibrary.Delay` 2.0)
  (`self.Hunt`))

(event `self.Sphere.OnComponentHit`
  (params (HitComponent :type "PrimitiveComponent Object Reference") (OtherActor :type "Actor Object Reference") (OtherComp :type "PrimitiveComponent Object Reference") (NormalImpulse :type "Vector Structure") (Hit :type "HitResult Structure (by ref)"))
  (bind _asbp_pacman (cast `/Game/Pacman/Blueprints/BP_Pacman` OtherActor))
  (`self.K2_SetActorLocation` _asbp_pacman (10000.0 10000.0 0.0) false false)
  (`self.Idle`)
  (`KismetSystemLibrary.Delay` 2.0)
  (`GameplayStatics.OpenLevel` "Level_01"))

(fn `UpdateMovementTarget`
  (locals (`AI Controller` :type "AIController Object Reference"))
  (set `local.AI Controller` (`AIBlueprintHelperLibrary.GetAIController` (`self.GetController`)))
  (switch `EEnemyState` (`self.State`)
    (:`Default`
      (`AIController.MoveToActor` (`local.AI Controller`) (`GameplayStatics.GetPlayerPawn` 0) -1.0 false true true null true))
    (:`Idle`
      (`Controller.StopMovement` (`local.AI Controller`)))))

(fn `UserConstructionScript`)